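; Combat component for the third-person player character, handling target lock and a sword combo attack.
; Target lock sphere-traces for a pawn using the camera, attaches a marker actor, switches to strafe movement and steers control rotation toward the target each Tick.
; Attack input plays a combo montage that stops at a notify unless another press was buffered.
; Begin/End hitbox events toggle a looping timer that sphere-traces the blade, applying damage with a brief cooldown.
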(event `self.ReceiveBeginPlay`
  ;[1 1 1] Get Player Class
  (bind _asbp_third_person_character (cast `/Game/ThirdPerson/Blueprints/BP_ThirdPersonCharacter` (`self.GetOwner`)))
  (set `self.Player BP` _asbp_third_person_character))

(event `EnhancedInput|/Game/ThirdPerson/Input/Actions/IA_TargetLock`
  (params (ActionValue :type Boolean) (ElapsedSeconds :type "Float (double-precision)") (TriggeredSeconds :type "Float (double-precision)") (InputAction :type "InputAction Object Reference" :default "/Game/ThirdPerson/Input/Actions/IA_TargetLock.IA_TargetLock"))
  (bind _returnvalue (`Actor.GetTransform` (`self.TargetLock Actor`)))
  (bind _transformcomponent (`PlayerCameraManager.TransformComponent` (`GameplayStatics.GetPlayerCameraManager` 0)))
  (bind _charactermovement (`Character.CharacterMovement` (`self.Player BP`)))
  (bind _charactermovement_2 (`Character.CharacterMovement` (`self.Player BP`)))
  (bind (_returnvalue_x _returnvalue_y _returnvalue_z) (`KismetMathLibrary.BreakVector` (`SceneComponent.K2_GetComponentLocation` _transformcomponent)))
  ;[0.9831 0.4398 1] Target Lock
  (:`Started`
    (`self.TargetLock Actor`
      (:`then`
        ;;[0.4621 0.807 1] Unuse StrafeMovement
        (set `self.TargetLock Actor` null)
        (set `CharacterMovementComponent.bOrientRotationToMovement` true _charactermovement_2)
        (set `CharacterMovementComponent.bUseControllerDesiredRotation` false _charactermovement_2)
        ;;[0.3515 1 0.3916] Unlock Widget
        (`Actor.K2_DestroyActor` (`self.TargetLock Widget`)))
      (:`else`
        (bind (_outhit _returnvalue_2) (`KismetSystemLibrary.SphereTraceSingleForObjects` :`End` (+ (`KismetMathLibrary.MakeVector` _returnvalue_x _returnvalue_y (+ _returnvalue_z 20.0)) (* (`KismetMathLibrary.GetForwardVector` (`SceneComponent.K2_GetComponentRotation` _transformcomponent)) 1000.0)) :`Radius` 150.0 :`ObjectTypes` (`|MakeArray` "ObjectTypeQuery3" :!type "EObjectTypeQuery Enum") :`DrawDebugType` "ForDuration" :`DrawTime` 2.0))
        (if _returnvalue_2
          ;;[0.4621 0.807 1] Use StrafeMovement
          (set `self.TargetLock Actor` (`.HitActor` (`GameplayStatics.BreakHitResult` _outhit)))
          (set `CharacterMovementComponent.bOrientRotationToMovement` false _charactermovement)
          (set `CharacterMovementComponent.bUseControllerDesiredRotation` true _charactermovement)
          ;;[0.3515 1 0.3916] TargetLock Widget
          (bind _returnvalue_3 (`|SpawnActorFromClass` "/Game/Blueprints/BP_TargetLock.BP_TargetLock_C" (`KismetMathLibrary.MakeTransform` (`KismetMathLibrary.MakeVector` (.x (.location _returnvalue)) (.y (.location _returnvalue)) (+ (.z (.location _returnvalue)) 20.0)) (.rotation _returnvalue) (.scale _returnvalue)) "AlwaysSpawn" "MultiplyWithRoot" null null))
          (bind _output_get (set `self.TargetLock Widget` _returnvalue_3))
          (`Actor.K2_AttachToActor` _output_get (`self.TargetLock Actor`) "None" "SnapToTarget" "SnapToTarget" "SnapToTarget" true))))))

(event `self.ReceiveTick`
  (params (DeltaSeconds :type "Float (single-precision)"))
  (bind (_returnvalue_roll _returnvalue_pitch _returnvalue_yaw) (`KismetMathLibrary.BreakRotator` (`KismetMathLibrary.FindLookAtRotation` (`Actor.K2_GetActorLocation` (`self.Player BP`)) (`Actor.K2_GetActorLocation` (`self.TargetLock Actor`)))))
  ;[0.9831 0.4398 1] Target Lock
  ;;[1 0.4891 0.555] CameraFacingLocation (TargetLock Update)
  (`self.TargetLock Actor`
    (:`then`
      (`Controller.SetControlRotation` (`Pawn.GetController` (`self.Player BP`)) (`KismetMathLibrary.MakeRotator` _returnvalue_roll (+ _returnvalue_pitch -20.0) _returnvalue_yaw)))
    (:`else`)))

(event `EnhancedInput|/Game/ThirdPerson/Input/Actions/IA_Attack`
  (params (ActionValue :type Boolean) (ElapsedSeconds :type "Float (double-precision)") (TriggeredSeconds :type "Float (double-precision)") (InputAction :type "InputAction Object Reference" :default "/Game/ThirdPerson/Input/Actions/IA_Attack.IA_Attack"))
  ;[1 0.04329 0] Sword Combo Animation
  (:`Started`
    (if (not (`self.isAttacking`))
      (set `self.isAttacking` true)
      (`|PlayMontage` (`Character.Mesh` (`self.Player BP`)) "/Game/Locomotion/Combat/SwordAttackCombo_Montage.SwordAttackCombo_Montage"
        (:`OnCompleted`
          (set `self.isAttacking` false :!label _label)
          (set `self.isCombo` false))
        (:`OnInterrupted`
          (goto _label))
        (:`OnNotifyBegin`
          (if (and (`self.isAttacking`) (`self.isCombo`))
            (set `self.isCombo` false)
            (else
              (`AnimInstance.Montage_Stop` (`SkeletalMeshComponent.GetAnimInstance` (`Character.Mesh` (`self.Player BP`))) 0.0 null)))))
      (else
        (set `self.isCombo` true)))))

(event `EndDamageHitbox`
  ;[1 0.6759 0.2471] Sword Hitbox
  (if (`KismetSystemLibrary.K2_IsValidTimerHandle` (stale `BeginDamageHitbox` _returnvalue))
    (`KismetSystemLibrary.K2_ClearAndInvalidateTimerHandle` (stale `BeginDamageHitbox` _returnvalue))))

(event `BeginDamageHitbox`
  ;[1 0.6759 0.2471] Sword Hitbox
  (bind _returnvalue (`KismetSystemLibrary.K2_SetTimerDelegate` (delegate `DamageHitbox`) 0.01 true)))

(event `DamageHitbox`
  (bind _player_bp (`self.Player BP`))
  ;[1 0.6759 0.2471] Sword Hitbox
  (bind (_outhit _returnvalue) (`KismetSystemLibrary.SphereTraceSingleForObjects` :`Start` (`SceneComponent.K2_GetComponentLocation` (`/Game/ThirdPerson/Blueprints/BP_ThirdPersonCharacter.Start Hitbox` _player_bp)) :`End` (`SceneComponent.K2_GetComponentLocation` (`/Game/ThirdPerson/Blueprints/BP_ThirdPersonCharacter.End Hitbox` _player_bp)) :`Radius` 25.0 :`ObjectTypes` (`|MakeArray` "ObjectTypeQuery3" :!type "EObjectTypeQuery Enum") :`DrawDebugType` "ForOneFrame"))
  (if _returnvalue
    (`/Engine/EditorBlueprintResources/StandardMacros.DoOnce` false :!label _label_2
      (:`Completed`
        (`GameplayStatics.ApplyDamage` (`.HitActor` (`GameplayStatics.BreakHitResult` _outhit)) (`self.SwordDamage`))
        (`KismetSystemLibrary.Delay` 0.2)
        (goto _label_2 :!via `Reset`)))))