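; BP_DoorBig is a large door that swings automatically when anything overlaps its front or back box, opening in opposite directions for each side.
; A RotatingMovement component drives the swing, switched on at a fixed rate for Duration and then zeroed.
; Ending the overlap waits WaitingTime plus Duration, then runs the reverse rotation.
; Motion is purely timed, with no angle checks or overlap filtering.
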(event `self.BoxFront.OnComponentBeginOverlap`
  (params (OverlappedComponent :type "PrimitiveComponent Object Reference") (OtherActor :type "Actor Object Reference") (OtherComp :type "PrimitiveComponent Object Reference") (OtherBodyIndex :type Integer) (bFromSweep :type Boolean) (SweepResult :type "HitResult Structure (by ref)"))
  (bind _rotatingmovement (`self.RotatingMovement`))
  ;[0.04167 0.04167 0.04167] Open
  (set `RotatingMovementComponent.RotationRate` (struct :`Yaw` 75.0) _rotatingmovement)
  (`KismetSystemLibrary.Delay` (`self.Duration`))
  (set `RotatingMovementComponent.RotationRate` (struct) _rotatingmovement))

(event `self.BoxFront.OnComponentEndOverlap`
  (params (OverlappedComponent :type "PrimitiveComponent Object Reference") (OtherActor :type "Actor Object Reference") (OtherComp :type "PrimitiveComponent Object Reference") (OtherBodyIndex :type Integer))
  (bind _rotatingmovement (`self.RotatingMovement`))
  ;[0.04167 0.04167 0.04167] Open
  (`KismetSystemLibrary.Delay` (+ (`self.WaitingTime`) (`self.Duration`)))
  (set `RotatingMovementComponent.RotationRate` (struct :`Yaw` -75.0) _rotatingmovement)
  (`KismetSystemLibrary.Delay` (`self.Duration`))
  (set `RotatingMovementComponent.RotationRate` (struct) _rotatingmovement))

(event `self.BoxBack.OnComponentBeginOverlap`
  (params (OverlappedComponent :type "PrimitiveComponent Object Reference") (OtherActor :type "Actor Object Reference") (OtherComp :type "PrimitiveComponent Object Reference") (OtherBodyIndex :type Integer) (bFromSweep :type Boolean) (SweepResult :type "HitResult Structure (by ref)"))
  (bind _rotatingmovement (`self.RotatingMovement`))
  ;[0.03125 0.03125 0.03125] Close
  (set `RotatingMovementComponent.RotationRate` (struct :`Yaw` -75.0) _rotatingmovement)
  (`KismetSystemLibrary.Delay` (`self.Duration`))
  (set `RotatingMovementComponent.RotationRate` (struct) _rotatingmovement))

(event `self.BoxBack.OnComponentEndOverlap`
  (params (OverlappedComponent :type "PrimitiveComponent Object Reference") (OtherActor :type "Actor Object Reference") (OtherComp :type "PrimitiveComponent Object Reference") (OtherBodyIndex :type Integer))
  (bind _rotatingmovement (`self.RotatingMovement`))
  ;[0.03125 0.03125 0.03125] Close
  (`KismetSystemLibrary.Delay` (+ (`self.WaitingTime`) (`self.Duration`)))
  (set `RotatingMovementComponent.RotationRate` (struct :`Yaw` 75.0) _rotatingmovement)
  (`KismetSystemLibrary.Delay` (`self.Duration`))
  (set `RotatingMovementComponent.RotationRate` (struct) _rotatingmovement))

(fn `UserConstructionScript`)