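; Boat actor that floats up and travels away on a scripted path after the player presses F near it.
; Overlapping the Box enables player input and arms the F key, with no check on the overlapping actor.
; F starts a Timeline raising MBoat; delays chained off its Update show a PointLight, then start a second Timeline moving it along X.
; A further delay from that Update drops the boat far downward.
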(event `self.Box.OnComponentBeginOverlap`
  (params (OverlappedComponent :type "PrimitiveComponent Object Reference") (OtherActor :type "Actor Object Reference") (OtherComp :type "PrimitiveComponent Object Reference") (OtherBodyIndex :type Integer) (bFromSweep :type Boolean) (SweepResult :type "HitResult Structure (by ref)"))
  ;[0.2604 0.2604 0.2604] Press F to float
  (`self.EnableInput` (`GameplayStatics.GetPlayerController` 0))
  (set `self.IsPressF` true))

(event `Key|F`
  (params (Key :type "Key Structure"))
  ;[0.2604 0.2604 0.2604] Press F to float
  (:`Pressed`
    (if (`self.IsPressF`)
      (bind (_direction _float) (`Timeline|Timeline`)
        (:`Update`
          (`SceneComponent.K2_SetRelativeLocation` (`self.M_Boat`) (`KismetMathLibrary.VLerp` (620.0 0.0 -200.0) (620.0 0.0 -15.0) _float) false false)
          (`KismetSystemLibrary.Delay` 2.5)
          (`SceneComponent.SetVisibility` (`self.PointLight`) true false)
          ;[0.125 0.125 0.125] Move
          (`KismetSystemLibrary.Delay` 5.0)
          (bind (_direction_2 _move) (`Timeline|Timeline_2`)
            (:`Update`
              (`SceneComponent.K2_SetRelativeLocation` (`self.M_Boat`) (`KismetMathLibrary.VLerp` (620.0 0.0 -15.0) (12250.0 0.0 -15.0) _move) false false)
              (`KismetSystemLibrary.Delay` 10.0)
              (`SceneComponent.K2_AddWorldOffset` (`self.M_Boat`) (0.0 0.0 -1000.0) false false))))))))

(fn `UserConstructionScript`)