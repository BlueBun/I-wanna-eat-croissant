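; Sliding door Blueprint that stays locked until its statue, acting as the key, is hit.
; A hit on the statue sets the Key flag and drops the statue far below out of the way.
; With Key set, overlapping the Box plays a Timeline that slides the door sideways; leaving reverses it after a delay.
; The construction script positions the statue from the NewLocation variable.
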(event `self.Box.OnComponentBeginOverlap`
  (params (OverlappedComponent :type "PrimitiveComponent Object Reference") (OtherActor :type "Actor Object Reference") (OtherComp :type "PrimitiveComponent Object Reference") (OtherBodyIndex :type Integer) (bFromSweep :type Boolean) (SweepResult :type "HitResult Structure (by ref)"))
  (if (`self.Key`)
    (bind (_direction _speed) (`Timeline|Timeline` :!label _label)
      (:`Update`
        (`SceneComponent.K2_SetRelativeLocation` (`self.SM_Door`) (`KismetMathLibrary.VLerp` (0.0 0.0 0.0) (0.0 200.0 0.0) _speed) false false)))))

(event `self.Box.OnComponentEndOverlap`
  (params (OverlappedComponent :type "PrimitiveComponent Object Reference") (OtherActor :type "Actor Object Reference") (OtherComp :type "PrimitiveComponent Object Reference") (OtherBodyIndex :type Integer))
  (`KismetSystemLibrary.Delay` 3.0)
  (goto _label :!via `Reverse`))

(event `self.SM_Statue.OnComponentHit`
  (params (HitComponent :type "PrimitiveComponent Object Reference") (OtherActor :type "Actor Object Reference") (OtherComp :type "PrimitiveComponent Object Reference") (NormalImpulse :type "Vector Structure") (Hit :type "HitResult Structure (by ref)"))
  ;[0.1302 0.1302 0.1302] Hit Key It's move to underworld
  (set `self.Key` true)
  (`SceneComponent.K2_AddWorldOffset` (`self.SM_Statue`) (0.0 0.0 -1000.0) false false))

(fn `UserConstructionScript`
  (`SceneComponent.K2_SetRelativeLocation` (`self.SM_Statue`) (`self.New Location`) false false))