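; BP_MoonHouse is a moon house actor that raises a bridge in sections when anything overlaps its trigger box.
; Overlap shows a text render, waits briefly, then plays timelines that lerp the bridge pieces and a rail upward.
; Each timeline's Update starts the next through a short Delay, staggering the rise into a cascade.
; Leaving the box hides the text after a delay but leaves the bridge timelines untouched.
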(event `self.Box.OnComponentBeginOverlap`
  (params (OverlappedComponent :type "PrimitiveComponent Object Reference") (OtherActor :type "Actor Object Reference") (OtherComp :type "PrimitiveComponent Object Reference") (OtherBodyIndex :type Integer) (bFromSweep :type Boolean) (SweepResult :type "HitResult Structure (by ref)"))
  (if true
    (`SceneComponent.SetVisibility` (`self.TextRender`) true false)
    (`KismetSystemLibrary.Delay` 2.0)
    (bind (_direction _float) (`Timeline|Timeline`)
      (:`Update`
        (`SceneComponent.K2_SetRelativeLocation` (`self.M_Bridge`) (`KismetMathLibrary.VLerp` (459.148902 -172.999999 -200.0) (459.148902 -172.999999 0.0) _float) false false)
        (`KismetSystemLibrary.Delay` 0.2)
        (bind (_direction_2 _float_2) (`Timeline|Timeline_0`)
          (:`Update`
            (`SceneComponent.K2_SetRelativeLocation` (`self.M_Bridge1`) (`KismetMathLibrary.VLerp` (1451.852126 -173.000001 -200.0) (1451.852126 -173.000001 0.0) _float_2) false false)
            (`KismetSystemLibrary.Delay` 0.2)
            (bind (_direction_3 _float_3) (`Timeline|Timeline_1`)
              (:`Update`
                (`SceneComponent.K2_SetRelativeLocation` (`self.M_Bridge2`) (`KismetMathLibrary.VLerp` (2449.839451 -173.000001 -200.0) (2449.839451 -173.000001 0.0) _float_3) false false)
                (`KismetSystemLibrary.Delay` 0.2)
                (bind (_direction_4 _float_4) (`Timeline|Timeline_2`)
                  (:`Update`
                    (`SceneComponent.K2_SetRelativeLocation` (`self.M_BridgeRail`) (`KismetMathLibrary.VLerp` (3090.0 -328.470078 -235.963809) (3090.0 -328.470078 -35.0) _float_4) false false)
                    (`KismetSystemLibrary.Delay` 0.2)
                    (bind (_direction_5 _float_5) (`Timeline|Timeline_3`)
                      (:`Update`
                        (`SceneComponent.K2_SetRelativeLocation` (`self.M_Bridge3`) (`KismetMathLibrary.VLerp` (3723.265425 -173.000001 -200.0) (3723.265425 -173.000001 0.0) _float_5) false false)))))))))))))

(event `self.Box.OnComponentEndOverlap`
  (params (OverlappedComponent :type "PrimitiveComponent Object Reference") (OtherActor :type "Actor Object Reference") (OtherComp :type "PrimitiveComponent Object Reference") (OtherBodyIndex :type Integer))
  (`KismetSystemLibrary.Delay` 5.0)
  (`SceneComponent.SetVisibility` (`self.TextRender`) false false))

(fn `UserConstructionScript`)