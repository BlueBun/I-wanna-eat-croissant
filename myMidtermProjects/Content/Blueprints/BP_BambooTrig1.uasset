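; BP_BambooTrig1 is a bamboo pickup trigger that also removes a door blocker.
; Overlapping Box shows a text prompt and enables input, so E hides the mini bamboo and its lights and drops BoxDoor, its text and light far below.
; Leaving hides the prompt after a delay, but E stays active.
; Hitting BoxDoor briefly shows the door text and light.
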(event `self.Box.OnComponentBeginOverlap`
  (params (OverlappedComponent :type "PrimitiveComponent Object Reference") (OtherActor :type "Actor Object Reference") (OtherComp :type "PrimitiveComponent Object Reference") (OtherBodyIndex :type Integer) (bFromSweep :type Boolean) (SweepResult :type "HitResult Structure (by ref)"))
  ;[0.0625 0.0625 0.0625] Show Text E collect
  (if true
    (`SceneComponent.SetVisibility` (`self.TextRender`) true false)
    ;[0.3698 0.3698 0.3698] Press E to unseen Bamboo
    (`self.EnableInput` (`GameplayStatics.GetPlayerController` 0))
    (set `self.IsPressE` true)))

(event `Key|E`
  (params (Key :type "Key Structure"))
  ;[0.3698 0.3698 0.3698] Press E to unseen Bamboo
  (:`Pressed`
    (if (`self.IsPressE`)
      (`SceneComponent.SetVisibility` (`self.SpotLight`) false false)
      (`SceneComponent.SetVisibility` (`self.BambooMini`) false false)
      (`SceneComponent.SetVisibility` (`self.PointLight`) false false)
      (`SceneComponent.K2_AddWorldOffset` (`self.BoxDoor`) (0.0 0.0 -1000.0) false false)
      (`SceneComponent.K2_AddWorldOffset` (`self.PointLight1`) (0.0 0.0 -1000.0) false false)
      (`SceneComponent.K2_AddWorldOffset` (`self.TextRenderDoor`) (0.0 0.0 -1000.0) false false))))

(event `self.Box.OnComponentEndOverlap`
  (params (OverlappedComponent :type "PrimitiveComponent Object Reference") (OtherActor :type "Actor Object Reference") (OtherComp :type "PrimitiveComponent Object Reference") (OtherBodyIndex :type Integer))
  ;[0.0625 0.0625 0.0625] Show Text E collect
  (`KismetSystemLibrary.Delay` 5.0)
  (`SceneComponent.SetVisibility` (`self.TextRender`) false false))

(event `self.BoxDoor.OnComponentHit`
  (params (HitComponent :type "PrimitiveComponent Object Reference") (OtherActor :type "Actor Object Reference") (OtherComp :type "PrimitiveComponent Object Reference") (NormalImpulse :type "Vector Structure") (Hit :type "HitResult Structure (by ref)"))
  (bind _textrenderdoor (`self.TextRenderDoor`))
  (`SceneComponent.SetVisibility` _textrenderdoor true false)
  (`SceneComponent.SetVisibility` (`self.PointLight1`) true false)
  (`KismetSystemLibrary.Delay` 5.0)
  (`SceneComponent.SetVisibility` _textrenderdoor false false)
  (`SceneComponent.SetVisibility` (`self.PointLight1`) false false))

(fn `UserConstructionScript`)