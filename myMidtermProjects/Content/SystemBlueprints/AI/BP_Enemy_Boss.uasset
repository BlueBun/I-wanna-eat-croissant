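; BP_Enemy_Boss is the boss enemy, with its own health bar, a big attack and death handling.
; When the player character overlaps ShowBossHP, it creates a WBP_BossHP widget on screen, then a tick later passes its bar to BPCStats.
; BigAttack plays a montage and returns the result.
; Die disables movement, ragdolls the mesh and sets both IsDead and IsBossDead.
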(event `self.ReceiveBeginPlay`)

(event `/Game/SystemBlueprints/BPI_Damage.Die`
  (`CharacterMovementComponent.DisableMovement` (`self.CharacterMovement`))
  (`PrimitiveComponent.SetSimulatePhysics` (`self.Mesh`) true)
  (set `self.isDead` true)
  (set `self.isBossDead` true))

(event `self.ShowBossHP.OnComponentBeginOverlap`
  (params (OverlappedComponent :type "PrimitiveComponent Object Reference") (OtherActor :type "Actor Object Reference") (OtherComp :type "PrimitiveComponent Object Reference") (OtherBodyIndex :type Integer) (bFromSweep :type Boolean) (SweepResult :type "HitResult Structure (by ref)"))
  (cast `/Game/ThirdPerson/Blueprints/BP_ThirdPersonCharacter` OtherActor)
  (bind _returnvalue (`|GenericCreateObject` "/Game/UI/WBP_BossHP.WBP_BossHP_C"))
  (bind _output_get (set `self.Boss HP` _returnvalue))
  (`UserWidget.AddToViewport` _output_get 0)
  (`KismetSystemLibrary.DelayUntilNextTick`)
  (`/Game/SystemBlueprints/BPC_Stats.Set HP bar progression` (`self.BPC_Stats`) (`/Game/UI/WBP_BossHP.HPBar` (`self.Boss HP`))))

(fn `BigAttack`
  (returns (Duration :type "Float (double-precision)"))
  (bind _returnvalue (`self.PlayAnimMontage` "/Game/Locomotion/Combat/BigAttack_Montage.BigAttack_Montage"))
  (return _returnvalue))

(fn `UserConstructionScript`
  (`parent.UserConstructionScript`))