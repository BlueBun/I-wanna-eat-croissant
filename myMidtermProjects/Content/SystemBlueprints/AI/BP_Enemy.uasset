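; BP_Enemy is a melee enemy with a health bar widget driven by its BPCStats component, which also takes incoming damage.
; SwordAttack plays a combo montage, while Begin/EndSwordTrace toggle a looping timer that sphere-traces the blade and applies damage, throttled by a delayed DoOnce.
; PointDamageTrace delivers a separate radial hit with an explosion effect; BigAttack is an empty stub.
; Die ragdolls the mesh, then destroys the actor after a delay.
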(event `self.ReceiveBeginPlay`
  (bind _aswbp_enemy_hp (cast `/Game/UI/WBP_EnemyHP` (`WidgetComponent.GetWidget` (`self.Widget`))))
  (`/Game/SystemBlueprints/BPC_Stats.Set HP bar progression` (`self.BPC_Stats`) (`/Game/UI/WBP_EnemyHP.HPBar` _aswbp_enemy_hp)))

(event `self.ReceiveAnyDamage`
  (params (Damage :type "Float (single-precision)") (DamageType :type "DamageType Object Reference") (InstigatedBy :type "Controller Object Reference") (DamageCauser :type "Actor Object Reference"))
  (`/Game/SystemBlueprints/BPC_Stats.Increase Value` (`self.BPC_Stats`) "NewEnumerator0" (* Damage -1.0)))

(event `/Game/SystemBlueprints/BPI_Damage.End Sword Trace`
  ;[1 0.6759 0.2471] Sword Hitbox Trace
  (if (`KismetSystemLibrary.K2_IsValidTimerHandle` (stale `/Game/SystemBlueprints/BPI_Damage.Begin Sword Trace` _returnvalue))
    (`KismetSystemLibrary.K2_ClearAndInvalidateTimerHandle` (stale `/Game/SystemBlueprints/BPI_Damage.Begin Sword Trace` _returnvalue))))

(event `/Game/SystemBlueprints/BPI_Damage.Begin Sword Trace`
  ;[1 0.6759 0.2471] Sword Hitbox Trace
  (bind _returnvalue (`KismetSystemLibrary.K2_SetTimerDelegate` (delegate `Damage Trace`) 0.01 true)))

(event `Damage Trace`
  ;[1 0.6759 0.2471] Sword Hitbox Trace
  (if (not (`self.isDead`))
    (bind (_outhit _returnvalue) (`KismetSystemLibrary.SphereTraceSingleForObjects` :`Start` (`SceneComponent.K2_GetComponentLocation` (`self.Start Sword Trace Pos`)) :`End` (`SceneComponent.K2_GetComponentLocation` (`self.End sword trace Pos`)) :`Radius` 25.0 :`ObjectTypes` (`|MakeArray` "ObjectTypeQuery3" :!type "EObjectTypeQuery Enum") :`DrawDebugType` "ForOneFrame"))
    (if _returnvalue
      (`/Engine/EditorBlueprintResources/StandardMacros.DoOnce` false :!label _label
        (:`Completed`
          (bind (_bblockinghit _binitialoverlap _time _distance _location _impactpoint _normal _impactnormal _physmat _hitactor) (`GameplayStatics.BreakHitResult` _outhit))
          (`GameplayStatics.ApplyDamage` _hitactor (`self.Sword Damage`))
          (`GameplayStatics.SpawnEmitterAtLocation` "/Game/StarterContent/Particles/P_Explosion.P_Explosion" _location (struct) (1.0 1.0 1.0) true "AutoRelease")
          (`KismetSystemLibrary.Delay` 0.2)
          (goto _label :!via `Reset`))))))

(event `/Game/SystemBlueprints/BPI_Damage.Die`
  (`CharacterMovementComponent.DisableMovement` (`self.CharacterMovement`))
  (`PrimitiveComponent.SetSimulatePhysics` (`self.Mesh`) true)
  (set `self.isDead` true)
  (`KismetSystemLibrary.Delay` 5.0)
  (`self.K2_DestroyActor`))

(event `/Game/SystemBlueprints/BPI_Damage.Point Damage Trace`
  (bind _returnvalue (`SceneComponent.K2_GetComponentLocation` (`self.PointDamageTrace Pos`)))
  (bind (_outhit _returnvalue_2) (`KismetSystemLibrary.SphereTraceSingleForObjects` :`Start` _returnvalue :`End` _returnvalue :`Radius` (`self.PointAttackRadius`) :`ObjectTypes` (`|MakeArray` "ObjectTypeQuery3" :!type "EObjectTypeQuery Enum") :`DrawTime` 1.0))
  (`GameplayStatics.SpawnEmitterAtLocation` "/Game/StarterContent/Particles/P_Explosion.P_Explosion" _returnvalue)
  (if _returnvalue_2
    (`GameplayStatics.ApplyDamage` (`.HitActor` (`GameplayStatics.BreakHitResult` _outhit)) 20.0)))

(fn `BigAttack`
  (returns (Duration :type "Float (double-precision)"))
  (return 0.0))

(fn `SwordAttack`
  (returns (Duration :type "Float (double-precision)"))
  (bind _returnvalue (`self.PlayAnimMontage` "/Game/Locomotion/Combat/SwordAttackCombo_Montage.SwordAttackCombo_Montage"))
  (return _returnvalue))

(fn `UserConstructionScript`)