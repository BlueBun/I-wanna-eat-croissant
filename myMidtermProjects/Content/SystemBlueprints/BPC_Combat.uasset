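; Player combat component for BP_ThirdPersonCharacter, handling target lock, sword combos, dodging, healing and an ultimate-charged transform.
; Target lock sphere-traces from the camera, attaches a marker, switches to strafing and steers control rotation each Tick.
; Montage notifies stop the combo unless another press was buffered, while a looping timer sphere-traces the sword for throttled damage.
; Attacks and directional dodges spend BPCStats stamina and pause its regen; hits build ultimate charge.
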(event `self.ReceiveBeginPlay`
  ;[1 1 1] Get Player Class
  (bind _asbp_third_person_character (cast `/Game/ThirdPerson/Blueprints/BP_ThirdPersonCharacter` (`self.GetOwner`)))
  (set `self.Player BP` _asbp_third_person_character))

(event `EnhancedInput|/Game/ThirdPerson/Input/Actions/IA_TargetLock`
  (params (ActionValue :type Boolean) (ElapsedSeconds :type "Float (double-precision)") (TriggeredSeconds :type "Float (double-precision)") (InputAction :type "InputAction Object Reference" :default "/Game/ThirdPerson/Input/Actions/IA_TargetLock.IA_TargetLock"))
  (bind _returnvalue (`Actor.GetTransform` (`self.TargetLock Actor`)))
  (bind _transformcomponent (`PlayerCameraManager.TransformComponent` (`GameplayStatics.GetPlayerCameraManager` 0)))
  (bind _charactermovement (`Character.CharacterMovement` (`self.Player BP`)))
  (bind _charactermovement_2 (`Character.CharacterMovement` (`self.Player BP`)))
  (bind (_returnvalue_x _returnvalue_y _returnvalue_z) (`KismetMathLibrary.BreakVector` (`SceneComponent.K2_GetComponentLocation` _transformcomponent)))
  ;[0.9831 0.4398 1] Target Lock
  (:`Started`
    (`self.TargetLock Actor`
      (:`then`
        ;;[0.4621 0.807 1] Unuse StrafeMovement
        (set `self.TargetLock Actor` null)
        (set `CharacterMovementComponent.bOrientRotationToMovement` true _charactermovement_2)
        (set `CharacterMovementComponent.bUseControllerDesiredRotation` false _charactermovement_2)
        ;;[0.3515 1 0.3916] Unlock Widget
        (`Actor.K2_DestroyActor` (`self.TargetLock Widget`)))
      (:`else`
        (bind (_outhit _returnvalue_2) (`KismetSystemLibrary.SphereTraceSingleForObjects` :`End` (+ (`KismetMathLibrary.MakeVector` _returnvalue_x _returnvalue_y (+ _returnvalue_z 20.0)) (* (`KismetMathLibrary.GetForwardVector` (`SceneComponent.K2_GetComponentRotation` _transformcomponent)) 1000.0)) :`Radius` 150.0 :`ObjectTypes` (`|MakeArray` "ObjectTypeQuery3" :!type "EObjectTypeQuery Enum") :`DrawDebugType` "ForDuration" :`DrawTime` 2.0))
        (if _returnvalue_2
          ;;[0.4621 0.807 1] Use StrafeMovement
          (set `self.TargetLock Actor` (`.HitActor` (`GameplayStatics.BreakHitResult` _outhit)))
          (set `CharacterMovementComponent.bOrientRotationToMovement` false _charactermovement)
          (set `CharacterMovementComponent.bUseControllerDesiredRotation` true _charactermovement)
          ;;[0.3515 1 0.3916] TargetLock Widget
          (bind _returnvalue_3 (`|SpawnActorFromClass` "/Game/SystemBlueprints/BP_TargetLockWidget.BP_TargetLockWidget_C" (`KismetMathLibrary.MakeTransform` (`KismetMathLibrary.MakeVector` (.x (.location _returnvalue)) (.y (.location _returnvalue)) (+ (.z (.location _returnvalue)) 20.0)) (.rotation _returnvalue) (.scale _returnvalue)) "AlwaysSpawn" "MultiplyWithRoot" null null))
          (bind _output_get (set `self.TargetLock Widget` _returnvalue_3))
          (`Actor.K2_AttachToActor` _output_get (`self.TargetLock Actor`) "None" "SnapToTarget" "SnapToTarget" "SnapToTarget" true))))))

(event `self.ReceiveTick`
  (params (DeltaSeconds :type "Float (single-precision)"))
  (bind (_returnvalue_roll _returnvalue_pitch _returnvalue_yaw) (`KismetMathLibrary.BreakRotator` (`KismetMathLibrary.FindLookAtRotation` (`Actor.K2_GetActorLocation` (`self.Player BP`)) (`Actor.K2_GetActorLocation` (`self.TargetLock Actor`)))))
  ;[0.9831 0.4398 1] Target Lock
  ;;[1 0.4891 0.555] CameraFacingLocation (TargetLock Update)
  (`self.TargetLock Actor`
    (:`then`
      (`Controller.SetControlRotation` (`Pawn.GetController` (`self.Player BP`)) (`KismetMathLibrary.MakeRotator` _returnvalue_roll (+ _returnvalue_pitch -20.0) _returnvalue_yaw)))
    (:`else`)))

(event `EnhancedInput|/Game/ThirdPerson/Input/Actions/IA_Attack`
  (params (ActionValue :type Boolean) (ElapsedSeconds :type "Float (double-precision)") (TriggeredSeconds :type "Float (double-precision)") (InputAction :type "InputAction Object Reference" :default "/Game/ThirdPerson/Input/Actions/IA_Attack.IA_Attack"))
  (bind _bpc_stats (`/Game/ThirdPerson/Blueprints/BP_ThirdPersonCharacter.BPC_Stats` (`self.Player BP`)))
  ;[1 0.04329 0] Attack Combo Animation
  (:`Started`
    (if (and (not (`self.isAttacking`)) (>= (`/Game/SystemBlueprints/BPC_Stats.Stamina` (`/Game/ThirdPerson/Blueprints/BP_ThirdPersonCharacter.BPC_Stats` (`self.Player BP`))) 10.0))
      (set `self.isAttacking` true)
      (`|PlayMontage` (`Character.Mesh` (`self.Player BP`)) "/Game/Locomotion/Combat/SwordAttackCombo_Montage.SwordAttackCombo_Montage"
        (:`then`
          (set `/Game/SystemBlueprints/BPC_Stats.isRegenStamina` false _bpc_stats)
          (`/Game/SystemBlueprints/BPC_Stats.Increase Value` _bpc_stats "NewEnumerator1" -10.0))
        (:`OnCompleted`
          (set `self.isAttacking` false :!label _label)
          (set `self.isCombo` false)
          (set `/Game/SystemBlueprints/BPC_Stats.isRegenStamina` true (`/Game/ThirdPerson/Blueprints/BP_ThirdPersonCharacter.BPC_Stats` (`self.Player BP`))))
        (:`OnInterrupted`
          (goto _label))
        (:`OnNotifyBegin`
          (if (and (`self.isAttacking`) (`self.isCombo`))
            (set `self.isCombo` false)
            (else
              (`AnimInstance.Montage_Stop` (`SkeletalMeshComponent.GetAnimInstance` (`Character.Mesh` (`self.Player BP`))) 0.0 "/Game/Locomotion/Combat/SwordAttackCombo_Montage.SwordAttackCombo_Montage")))))
      (else
        (set `self.isCombo` true)))))

(event `End DamageTrace`
  ;[1 0.6759 0.2471] Sword Hitbox Trace
  (if (`KismetSystemLibrary.K2_IsValidTimerHandle` (stale `Begin DamageTrace` _returnvalue))
    (`KismetSystemLibrary.K2_ClearAndInvalidateTimerHandle` (stale `Begin DamageTrace` _returnvalue))))

(event `Begin DamageTrace`
  ;[1 0.6759 0.2471] Sword Hitbox Trace
  (bind _returnvalue (`KismetSystemLibrary.K2_SetTimerDelegate` (delegate `Damage Trace`) 0.01 true)))

(event `Damage Trace`
  (bind _player_bp (`self.Player BP`))
  ;[1 0.6759 0.2471] Sword Hitbox Trace
  (bind (_outhit _returnvalue) (`KismetSystemLibrary.SphereTraceSingleForObjects` (`SceneComponent.K2_GetComponentLocation` (`/Game/ThirdPerson/Blueprints/BP_ThirdPersonCharacter.Start Sword Trace Pos` _player_bp)) (`SceneComponent.K2_GetComponentLocation` (`/Game/ThirdPerson/Blueprints/BP_ThirdPersonCharacter.End sword trace Pos` _player_bp)) 25.0 (`|MakeArray` "ObjectTypeQuery3" :!type "EObjectTypeQuery Enum")))
  (if _returnvalue
    (`/Engine/EditorBlueprintResources/StandardMacros.DoOnce` false :!label _label_2
      (:`Completed`
        (bind (_bblockinghit _binitialoverlap _time _distance _location _impactpoint _normal _impactnormal _physmat _hitactor) (`GameplayStatics.BreakHitResult` _outhit))
        (`GameplayStatics.ApplyDamage` _hitactor (`self.SwordDamage`))
        (`GameplayStatics.SpawnEmitterAtLocation` "/Game/StarterContent/Particles/P_Explosion.P_Explosion" _location (struct) (0.1 0.1 0.1) true "AutoRelease")
        (`/Game/SystemBlueprints/BPC_Stats.Increase Value` (`/Game/ThirdPerson/Blueprints/BP_ThirdPersonCharacter.BPC_Stats` (`self.Player BP`)) "NewEnumerator2" 10.0)
        (`KismetSystemLibrary.Delay` 0.2)
        (goto _label_2 :!via `Reset`)))))

(event `EnhancedInput|/Game/ThirdPerson/Input/Actions/IA_Dodge`
  (params (ActionValue :type Boolean) (ElapsedSeconds :type "Float (double-precision)") (TriggeredSeconds :type "Float (double-precision)") (InputAction :type "InputAction Object Reference" :default "/Game/ThirdPerson/Input/Actions/IA_Dodge.IA_Dodge"))
  (bind _bpc_stats (`/Game/ThirdPerson/Blueprints/BP_ThirdPersonCharacter.BPC_Stats` (`self.Player BP`)))
  ;[0.1209 0.5279 1] Dodging
  (:`Started`
    (if (and (not (`self.isDodging`)) (>= (`/Game/SystemBlueprints/BPC_Stats.Stamina` (`/Game/ThirdPerson/Blueprints/BP_ThirdPersonCharacter.BPC_Stats` (`self.Player BP`))) 20.0))
      (set `self.isDodging` true)
      (`|ExecutionSequence`
        (:`then_0`
          (if (`CharacterMovementComponent.bUseControllerDesiredRotation` (`Character.CharacterMovement` (`self.Player BP`)))
            (switch `string` (`KismetTextLibrary.Conv_TextToString` (`KismetInputLibrary.Key_GetDisplayName` (`/Game/ThirdPerson/Blueprints/BP_ThirdPersonCharacter.Direction Key` (`self.Player BP`))))
              (:`W`
                (set `self.MovementDirection` "NewEnumerator0"))
              (:`A`
                (set `self.MovementDirection` "NewEnumerator2"))
              (:`S`
                (set `self.MovementDirection` "NewEnumerator1"))
              (:`D`
                (set `self.MovementDirection` "NewEnumerator3")))
            (else
              (set `self.MovementDirection` "NewEnumerator0"))))
        (:`then_1`
          (`|PlayMontage` (`Character.Mesh` (`self.Player BP`)) (select `/Game/SystemBlueprints/E_MovementDirection` (`self.MovementDirection`) :`NewEnumerator0` "/Game/Locomotion/Combat/Dodging/Dodge_F_Montage.Dodge_F_Montage" :`NewEnumerator1` "/Game/Locomotion/Combat/Dodging/Dodge_B_Montage.Dodge_B_Montage" :`NewEnumerator2` "/Game/Locomotion/Combat/Dodging/Dodge_L_Montage.Dodge_L_Montage" :`NewEnumerator3` "/Game/Locomotion/Combat/Dodging/Dodge_R_Montage.Dodge_R_Montage" :!type "AnimMontage Object Reference")
            (:`then`
              (set `/Game/SystemBlueprints/BPC_Stats.isRegenStamina` false _bpc_stats)
              (`/Game/SystemBlueprints/BPC_Stats.Increase Value` _bpc_stats "NewEnumerator1" -20.0))
            (:`OnCompleted`
              (set `self.isDodging` false :!label _label_3)
              (set `/Game/SystemBlueprints/BPC_Stats.isRegenStamina` true (`/Game/ThirdPerson/Blueprints/BP_ThirdPersonCharacter.BPC_Stats` (`self.Player BP`))))
            (:`OnInterrupted`
              (goto _label_3))))))))

(event `EnhancedInput|/Game/ThirdPerson/Input/Actions/IA_Heal`
  (params (ActionValue :type Boolean) (ElapsedSeconds :type "Float (double-precision)") (TriggeredSeconds :type "Float (double-precision)") (InputAction :type "InputAction Object Reference" :default "/Game/ThirdPerson/Input/Actions/IA_Heal.IA_Heal"))
  ;[1 1 1] press E to heal
  (:`Started`
    (`/Game/SystemBlueprints/BPC_Stats.Increase Value` (`/Game/ThirdPerson/Blueprints/BP_ThirdPersonCharacter.BPC_Stats` (`self.Player BP`)) "NewEnumerator0" 30.0)))

(event `EnhancedInput|/Game/ThirdPerson/Input/Actions/IA_Transform`
  (params (ActionValue :type Boolean) (ElapsedSeconds :type "Float (double-precision)") (TriggeredSeconds :type "Float (double-precision)") (InputAction :type "InputAction Object Reference" :default "/Game/ThirdPerson/Input/Actions/IA_Transform.IA_Transform"))
  (bind _bpc_stats (`/Game/ThirdPerson/Blueprints/BP_ThirdPersonCharacter.BPC_Stats` (`self.Player BP`)))
  ;[1 0.1424 0.7152] Transform
  (:`Started`
    (if (>= (`/Game/SystemBlueprints/BPC_Stats.UltimateCharge` _bpc_stats) (`/Game/SystemBlueprints/BPC_Stats.maxUltimateCharge` _bpc_stats))
      (set `/Game/SystemBlueprints/BPC_Stats.isCharging` false (`/Game/ThirdPerson/Blueprints/BP_ThirdPersonCharacter.BPC_Stats` (`self.Player BP`)))
      (set `self.SwordDamage` 750.0)
      (`PrimitiveComponent.SetMaterial` (`/Game/ThirdPerson/Blueprints/BP_ThirdPersonCharacter.Sword` (`self.Player BP`)) 0 "/Game/StarterContent/Materials/New/M_Neon_Red.M_Neon_Red")
      (`PrimitiveComponent.SetMaterial` (`Character.Mesh` (`self.Player BP`)) 0 "/Game/StarterContent/Materials/New/M_Neon_Pink.M_Neon_Pink"))))